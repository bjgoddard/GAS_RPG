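; BP_SlingshotRock is a rock actor in the enemy ability set, by its name a slingshot projectile, with a tumbling mesh.
; BeginPlay randomizes yaw, pitch and roll rates, then sets the sphere collision to query-only after a short delay.
; Tick rotates the mesh locally, scaling yaw by delta time, while pitch and roll use their squared rates, making them frame-rate dependent and never negative.
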(event EventBeginPlay
  (bind _returnvalue (Math|Random|RandomFloatinRange -5e+02 5e+02))
  (Variables|Default|SetYaw%20Rotation%20Rate _returnvalue)
  (Variables|Default|SetPitch%20Rotation%20Rate _returnvalue)
  (Variables|Default|SetRoll%20Rotation%20Rate _returnvalue)
  (Utilities|FlowControl|Delay 0.1)
  (Collision|SetCollisionEnabled (Variables|Default|GetSphere) "QueryOnly"))

(event Collision|EventActorBeginOverlap
  (params (OtherActor :type Actor%20Object%20Reference)))

(event EventTick
  (params (DeltaSeconds :type Float%20%28single-precision%29))
  (bind _pitch_rotation_rate (Variables|Default|GetPitch%20Rotation%20Rate))
  (bind _roll_rotation_rate (Variables|Default|GetRoll%20Rotation%20Rate))
  (Transformation|AddLocalRotation (Variables|Default|GetRockMesh) (Math|Rotator|MakeRotator (* _roll_rotation_rate _roll_rotation_rate) (* _pitch_rotation_rate _pitch_rotation_rate) (* DeltaSeconds (Variables|Default|GetYaw%20Rotation%20Rate))) false false))

(fn ConstructionScript)